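; BP_Alaria is the Alaria destination actor: it reveals itself on the fog of war and serves as the win trigger.
; On BeginPlay, a vertical complex trace at its location yields a collision UV, which feeds an exploring material drawn into the FogOfWar render target.
; Any overlap with its Box prints an arrival message and, after a delay, shows the win screen widget, without checking which actor entered.
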(event OnComponentHit(Cube)
  (params (HitComponent :type Primitive%20Component%20Object%20Reference) (OtherActor :type Actor%20Object%20Reference) (OtherComp :type Primitive%20Component%20Object%20Reference) (NormalImpulse :type Vector :default "0, 0, 0") (Hit :type Hit%20Result%20Structure%20%28by%20ref%29)))

(event OnComponentBeginOverlap(Cube)
  (params (OverlappedComponent :type Primitive%20Component%20Object%20Reference) (OtherActor :type Actor%20Object%20Reference) (OtherComp :type Primitive%20Component%20Object%20Reference) (OtherBodyIndex :type Integer) (bFromSweep :type Boolean) (SweepResult :type Hit%20Result%20Structure%20%28by%20ref%29)))

(event OnClicked(Cube)
  (params (TouchedComponent :type Primitive%20Component%20Object%20Reference) (ButtonPressed :type Key%20Structure :default "None")))

(event OnComponentBeginOverlap(Box)
  (params (OverlappedComponent :type Primitive%20Component%20Object%20Reference) (OtherActor :type Actor%20Object%20Reference) (OtherComp :type Primitive%20Component%20Object%20Reference) (OtherBodyIndex :type Integer) (bFromSweep :type Boolean) (SweepResult :type Hit%20Result%20Structure%20%28by%20ref%29))
  (Development|PrintString "you've reached Alaria!" true true "(R=1.000000,G=0.000000,B=0.165844,A=1.000000)" 4.0)
  (Utilities|FlowControl|Delay 5.0)
  (bind _returnvalue (UserInterface|CreateWidget "/Game/UIUX/UI_WinScreen.UI_WinScreen_C"))
  (UserInterface|Viewport|AddtoViewport _returnvalue 0))

(event EventBeginPlay
  (bind _returnvalue (Transformation|GetActorLocation))
  (bind _returnvalue_2 (Rendering|Material|CreateDynamicMaterialInstance "/Game/Blueprints/FogOfWar/FOW_Exploring_Mat.FOW_Exploring_Mat" "None" "None" :!class /Script/Engine.KismetMaterialLibrary))
  (Variables|Default|SetFOWMat _returnvalue_2)
  (bind _returnvalue_3 (Rendering|Material|CreateDynamicMaterialInstance "/Game/Blueprints/FogOfWar/FOW_Explored_Mat.FOW_Explored_Mat" "None" "None" :!class /Script/Engine.KismetMaterialLibrary))
  (Variables|Default|SetFOWExploredMat _returnvalue_3)
  (bind _outhit (Collision|LineTraceByChannel (+ _returnvalue "0.000000,0.000000,2000.000000") (+ _returnvalue "0.000000,0.000000,-2000.000000") "TraceTypeQuery3" true 0 "None"))
  (Rendering|Material|SetVectorParameterValue (Variables|Default|GetFOWMat) "Location" (Utilities|Struct|MakeLinearColor (.x (.UV (Class|GameplayStatics|FindCollisionUV _outhit))) (.y (.UV (Class|GameplayStatics|FindCollisionUV _outhit))) 0.0 1.0) :!class /Script/Engine.MaterialInstanceDynamic)
  (Rendering|DrawMaterialtoRenderTarget "/Game/Blueprints/FogOfWar/FogOfWar.FogOfWar" (Variables|Default|GetFOWMat)))

(event Collision|EventActorBeginOverlap
  (params (OtherActor :type Actor%20Object%20Reference)))

(event EventTick
  (params (DeltaSeconds :type Float%20%28single-precision%29)))

(fn ConstructionScript)