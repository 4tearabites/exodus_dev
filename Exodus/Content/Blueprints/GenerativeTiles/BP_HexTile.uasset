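; BP_HexTile is a generative hex tile actor that gives itself a random elevation.
; Its Construction Script picks a random normalized height between -1 and 1, then shifts the static mesh vertically by that height scaled by Strength plus Offset.
; The unscaled height also feeds the mesh materials' Elevation parameter, so shading can follow the displacement.
; The event graph holds only disabled placeholder events.
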(event EventBeginPlay)

(event Collision|EventActorBeginOverlap
  (params (OtherActor :type Actor%20Object%20Reference)))

(event EventTick
  (params (DeltaSeconds :type Float%20%28single-precision%29)))

(fn ConstructionScript
  (bind _staticmesh (Variables|Default|GetStaticMesh))
  (Variables|Default|SetHeight (Math|Random|RandomFloatinRange -1.0 1.0))
  (Transformation|SetWorldLocation _staticmesh (+ (Transformation|GetWorldLocation _staticmesh) (Math|Vector|MakeVector 0.0 0.0 (+ (* (Variables|Default|GetStrength) (Variables|Default|GetHeight)) (Variables|Default|GetOffset)))) false false)
  (Rendering|Material|SetScalarParameterValueonMaterials (Variables|Default|GetStaticMesh) "Elevation" (Variables|Default|GetHeight)))