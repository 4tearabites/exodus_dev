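; Collectible pickup actor whose mesh spins and bobs until an actor interacts with it.
; A timeline started on BeginPlay drives the yaw rotation and vertical bounce through two curves.
; Interact sets the timeline play rate from SpinTime, immediately destroys the actor, then decrements and prints the remaining item count on BP_ThirdPersonGameMode.
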(event EventBeginPlay
  (bind _staticmesh (Variables|Default|GetStaticMesh))
  (bind (_direction _medalanim _bouncecurve) (Timeline|medalSpin Play)
    (:Update
      (Transformation|SetRelativeRotation _staticmesh (Math|Rotator|MakeRotator 0.0 0.0 (Math|Float|Lerp 0.0 3.6e+02 _medalanim)) false false)
      (Transformation|SetRelativeLocation _staticmesh (Math|Vector|MakeVector 0.0 0.0 (Math|Float|Lerp -1e+01 1e+01 _bouncecurve)) false false))))

(event Collision|EventActorBeginOverlap
  (params (OtherActor :type Actor%20Object%20Reference)))

(event EventTick
  (params (DeltaSeconds :type Float%20%28single-precision%29)))

(fn ConstructionScript)

(fn Interact
  (params (InteractingActor :type Character%20Object%20Reference))
  (Components|Timeline|SetPlayRate (Variables|Default|GetmedalSpin) (/ 1.0 (Variables|Default|GetspinTime)))
  (Actor|DestroyActor)
  (bind _asbp_third_person_game_mode (Utilities|Casting|CastToBP_ThirdPersonGameMode (Game|GetGameMode)))
  (bind _result (Math|Integer|DecrementInt (Variables|/Game/ThirdPerson/Blueprints/BP_ThirdPersonGameMode.BP_ThirdPersonGameMode_C|GetitemsLeft _asbp_third_person_game_mode))
    (:%20%20
      (bind _output_get (Variables|/Game/ThirdPerson/Blueprints/BP_ThirdPersonGameMode.BP_ThirdPersonGameMode_C|SetitemsLeft _asbp_third_person_game_mode _result))
      (Development|PrintString (Utilities|String|ToString(Integer) _output_get))
      (return true))))