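; Procedural hex-tile terrain generator that builds a staggered grid and scatters Sprite_Camera actors over it at play.
; The construction script adds tiles as mesh instances, or as BP_HexTile child actors when not instanced.
; Two summed FastNoise layers set each instance's height and custom data, with a stretched instance beneath as a column.
; BeginPlay randomly picks recorded tiles and spawns a sprite at a random point on each.
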(event EventBeginPlay
  (bind _tilemesh (Variables|GridOptions|GetTileMesh))
  (bind _scale (Variables|GridOptions|GetScale))
  (bind _scale_2 (Variables|GridOptions|GetScale))
  (bind _tilemesh_2 (Variables|GridOptions|GetTileMesh))
  (bind _returnvalue (StaticMesh|GetBoundingBox _tilemesh_2))
  (bind _returnvalue_2 (StaticMesh|GetBoundingBox _tilemesh))
  (bind _returnvalue_3 (* (.y (.max _returnvalue)) _scale_2))
  (bind _returnvalue_4 (* (.x (.max _returnvalue_2)) _scale))
  (bind _returnvalue_5 (/ _returnvalue_4 2.0))
  (bind _returnvalue_6 (/ _returnvalue_3 2.0))
  (for (_array_element _array_index) (Variables|Default|GetInstace%20Indexes%20array)
    (if (Math|Random|RandomBool)
      ;[1 1 1] add png elements
      (Game|SpawnActorfromClass "/Game/Blueprints/Sprite_FaceCamera/Sprite_Camera.Sprite_Camera_C" (Math|Transform|MakeTransform (Math|Vector|MakeVector (Math|Random|RandomFloatinRange (- (.x (.location (.OutInstanceTransform (Components|InstancedStaticMesh|GetInstanceTransform (Variables|Default|GetInstancedStaticMesh) _array_element true)))) _returnvalue_5) (+ (.x (.location (.OutInstanceTransform (Components|InstancedStaticMesh|GetInstanceTransform (Variables|Default|GetInstancedStaticMesh) _array_element true)))) _returnvalue_5)) (Math|Random|RandomFloatinRange (- (.y (.location (.OutInstanceTransform (Components|InstancedStaticMesh|GetInstanceTransform (Variables|Default|GetInstancedStaticMesh) _array_element true)))) _returnvalue_6) (+ (.y (.location (.OutInstanceTransform (Components|InstancedStaticMesh|GetInstanceTransform (Variables|Default|GetInstancedStaticMesh) _array_element true)))) _returnvalue_6)) (.z (.location (.OutInstanceTransform (Components|InstancedStaticMesh|GetInstanceTransform (Variables|Default|GetInstancedStaticMesh) _array_element true))))) "0, 0, 0" (.scale (.OutInstanceTransform (Components|InstancedStaticMesh|GetInstanceTransform (Variables|Default|GetInstancedStaticMesh) _array_element true)))) "Undefined" "MultiplyWithRoot" 0 "NewEnumerator0" 0))))

(fn ConstructionScript
  (bind _noisescale (Variables|Lvl1NoiseSettings|GetNoiseScale))
  (bind _noisescale_lvl2 (Variables|Lvl2NoiseSettings|GetNoiseScale_Lvl2))
  ;[1 1 1] construct level 1 noise
  (bind _returnvalue (Game|ConstructObjectfromClass "/Script/FastNoiseGenerator.FastNoiseWrapper"))
  (bind _output_get (Variables|Default|SetNoiseWrapperLvl_1 _returnvalue))
  (Class|FastNoiseWrapper|SetupFastNoise _output_get (Variables|Lvl1noisesettings|GetNoise%20Type) (Variables|Lvl1NoiseSettings|GetSeed) (Variables|Lvl1NoiseSettings|GetFrequency) (Variables|Lvl1NoiseSettings|GetInterp) (Variables|Lvl1NoiseSettings|GetFractaltype) (Variables|Lvl1NoiseSettings|GetOctaves) (Variables|Lvl1NoiseSettings|GetLacunarity) (Variables|Lvl1NoiseSettings|GetGain) (Variables|Lvl1NoiseSettings|GetCellular%20Jitter) (Variables|Lvl1NoiseSettings|GetCellular%20Distance%20Function) (Variables|Lvl1NoiseSettings|GetCellular%20Return%20Type))
  ;[1 1 1] construct level 2 noise
  (bind _returnvalue_2 (Game|ConstructObjectfromClass "/Script/FastNoiseGenerator.FastNoiseWrapper"))
  (bind _output_get_2 (Variables|Default|SetNoiseWrapperLvl_2 _returnvalue_2))
  (Class|FastNoiseWrapper|SetupFastNoise _output_get_2 (Variables|Lvl2noisesettings|GetNoise%20Type_Lvl2) (Variables|Lvl2NoiseSettings|GetSeed_Lvl2) (Variables|Lvl2NoiseSettings|GetFrequency_Lvl2) (Variables|Lvl2NoiseSettings|GetInterp_Lvl2) (Variables|Lvl2NoiseSettings|GetFractaltype_Lvl2) (Variables|Lvl2NoiseSettings|GetOctaves_Lvl2) (Variables|Lvl2NoiseSettings|GetLacunarity_Lvl2) (Variables|Lvl2NoiseSettings|GetGain_Lvl2) (Variables|Lvl2NoiseSettings|GetCellular%20Jitter_Lvl2) (Variables|Lvl2NoiseSettings|GetCellular%20Distance%20Function_Lvl2) (Variables|Lvl2NoiseSettings|GetCellular%20Return%20Type_Lvl2))
  (Components|StaticMesh|SetStaticMesh (Variables|Default|GetInstancedStaticMesh) (Variables|GridOptions|GetTileMesh))
  (Variables|Default|SetRadius (* (.x (.max (StaticMesh|GetBoundingBox (Variables|GridOptions|GetTileMesh)))) (Variables|GridOptions|GetScale)))
  (for _index (range 0 (- (Variables|GridOptions|Gethight) 1))
    (for _index_2 (range 0 (- (Variables|GridOptions|Getwidth) 1))
      (if (Variables|GridOptions|GetInstanced?)
        (bind _returnvalue_3 (Components|InstancedStaticMesh|AddInstance (Variables|Default|GetInstancedStaticMesh) (Math|Transform|MakeTransform (Math|Vector|MakeVector (+ (* _index_2 2 (Variables|Default|GetRadius)) (* _index_2 (Variables|GridOptions|GetOffset)) (Variables|Default|GetRowOffset)) (+ (* (/ (* (Variables|Default|GetRadius) 2.0) (Math|Float|Sqrt 3.0)) 0.9 _index) (* _index (Variables|GridOptions|GetOffset))) 0.0) "0, 0, 0" (Math|Conversions|ToVector(Float) (Variables|GridOptions|GetScale))) false))
        (bind _output_get_3 (Variables|InstancedTileOptions|SetInstanced%20Index _returnvalue_3))
        (Utilities|Array|Add (Variables|Default|GetInstace%20Indexes%20array) _output_get_3)
        (Variables|Default|SetTileHeight (+ (Math|Float|Clamp(Float) (Class|FastNoiseWrapper|GetNoise2D (Variables|Default|GetNoiseWrapperLvl_2) (* (.x (.location (.OutInstanceTransform (Components|InstancedStaticMesh|GetInstanceTransform (Variables|Default|GetInstancedStaticMesh) (Variables|InstancedTileOptions|GetInstanced%20Index) false)))) _noisescale_lvl2) (* (.y (.location (.OutInstanceTransform (Components|InstancedStaticMesh|GetInstanceTransform (Variables|Default|GetInstancedStaticMesh) (Variables|InstancedTileOptions|GetInstanced%20Index) false)))) _noisescale_lvl2)) -1.0) (Class|FastNoiseWrapper|GetNoise2D (Variables|Default|GetNoiseWrapperLvl_1) (* (.x (.location (.OutInstanceTransform (Components|InstancedStaticMesh|GetInstanceTransform (Variables|Default|GetInstancedStaticMesh) (Variables|InstancedTileOptions|GetInstanced%20Index) false)))) _noisescale) (* (.y (.location (.OutInstanceTransform (Components|InstancedStaticMesh|GetInstanceTransform (Variables|Default|GetInstancedStaticMesh) (Variables|InstancedTileOptions|GetInstanced%20Index) false)))) _noisescale))))
        (Components|InstancedStaticMesh|UpdateInstanceTransform (Variables|Default|GetInstancedStaticMesh) (Variables|InstancedTileOptions|GetInstanced%20Index) (Math|Transform|MakeTransform (+ (.location (.OutInstanceTransform (Components|InstancedStaticMesh|GetInstanceTransform (Variables|Default|GetInstancedStaticMesh) (Variables|InstancedTileOptions|GetInstanced%20Index) true))) (Math|Vector|MakeVector 0.0 0.0 (+ (* (Variables|Default|GetTileHeight) (Variables|InstancedTileOptions|GetTileStregth)) (Variables|InstancedTileOptions|GetTileOffset)))) "0, 0, 0" (.scale (.OutInstanceTransform (Components|InstancedStaticMesh|GetInstanceTransform (Variables|Default|GetInstancedStaticMesh) (Variables|InstancedTileOptions|GetInstanced%20Index) true)))) false false false)
        (Utilities|Array|Add (Variables|Default|GetTile%20Heights%20array) (Variables|Default|GetTileHeight))
        (Components|InstancedStaticMesh|SetCustomDataValue (Variables|Default|GetInstancedStaticMesh) (Variables|InstancedTileOptions|GetInstanced%20Index) 0 (Variables|Default|GetTileHeight) true)
        (bind _returnvalue_4 (Components|InstancedStaticMesh|AddInstance (Variables|Default|GetInstancedStaticMesh) (Math|Transform|MakeTransform (- (.location (.OutInstanceTransform (Components|InstancedStaticMesh|GetInstanceTransform (Variables|Default|GetInstancedStaticMesh) (Variables|InstancedTileOptions|GetInstanced%20Index) true))) (Math|Vector|MakeVector 0.0 0.0 (* (Math|Float|Absolute(Float) (.z (.min (StaticMesh|GetBoundingBox (Variables|GridOptions|GetTileMesh))))) (Variables|GridOptions|GetScale)))) "0, 0, 0" (+ (Math|Conversions|ToVector(Float) (Variables|GridOptions|GetScale)) "0.000000,0.000000,10.000000")) true))
        (Variables|InstancedTileOptions|SetlowerInstanceIndex _returnvalue_4)
        (else
          (bind _returnvalue_5 (AddComponent|AddChildActorComponent false (Math|Transform|MakeTransform (Math|Vector|MakeVector (+ (* _index_2 2 (Variables|Default|GetRadius)) (* _index_2 (Variables|GridOptions|GetOffset)) (Variables|Default|GetRowOffset)) (+ (* (/ (* (Variables|Default|GetRadius) 2.0) (Math|Float|Sqrt 3.0)) 0.9 _index) (* _index (Variables|GridOptions|GetOffset))) 0.0) "0, 0, 0" (Math|Conversions|ToVector(Float) (Variables|GridOptions|GetScale)))))
          (ChildActorComponent|SetChildActorClass _returnvalue_5 "/Game/Blueprints/GenerativeTiles/BP_HexTile.BP_HexTile_C"))))
    (Utilities|FlowControl|FlipFlop
      (:A
        (Variables|Default|SetRowOffset (* (Variables|Default|GetRadius) -1.0)))
      (:B
        (Variables|Default|SetRowOffset 0.0)))))