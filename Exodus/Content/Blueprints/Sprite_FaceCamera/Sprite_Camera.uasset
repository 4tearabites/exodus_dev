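; Billboard sprite actor that shows a flat plane which turns to follow the player camera.
; On BeginPlay, the SpriteType selects the plane's material for wilderness, mountain or water, and wilderness sprites are also scaled up.
; Every tick, it computes the look-at rotation from camera to plane and applies offset roll and yaw with zero pitch as relative rotation, keeping the sprite upright.
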(event EventBeginPlay
  (bind _sprite_plane (Variables|Default|GetSprite_Plane))
  (bind _sprite_plane_2 (Variables|Default|GetSprite_Plane))
  (switch Utilities|FlowControl|Switch|SwitchonSpriteTypesEnum (Variables|Default|GetSpriteType)
    (:NewEnumerator0
      (Rendering|Material|SetMaterial _sprite_plane 0 "/Game/Blueprints/Tile_Textures/Asset_Textures/Materials/Tree_Material.Tree_Material")
      (Transformation|SetWorldScale3D _sprite_plane_2 (* (Transformation|GetWorldScale _sprite_plane_2) "2.000000,2.500000,2.000000")))
    (:NewEnumerator1
      (Rendering|Material|SetMaterial _sprite_plane 0 "/Game/Blueprints/Tile_Textures/Asset_Textures/Materials/Rock_Material.Rock_Material"))
    (:NewEnumerator3
      (Rendering|Material|SetMaterial _sprite_plane 0 "/Game/Blueprints/Sprite_FaceCamera/Test_Sprite.Test_Sprite"))))

(event EventTick
  (params (DeltaSeconds :type Float%20%28single-precision%29))
  (bind _returnvalue (Game|GetPlayerCameraManager 0))
  (bind _sprite_plane (Variables|Default|GetSprite_Plane))
  (bind _returnvalue_2 (Camera|GetCameraLocation _returnvalue))
  (bind _returnvalue_3 (Transformation|GetWorldLocation _sprite_plane))
  (bind _returnvalue_4 (Math|Rotator|FindLookatRotation _returnvalue_2 _returnvalue_3))
  (bind (_roll _pitch _yaw) (Math|Rotator|BreakRotator _returnvalue_4))
  (Transformation|SetRelativeRotation (Variables|Default|GetSprite_Plane) (Math|Rotator|MakeRotator (+ _roll 9e+01) 0.0 (+ _yaw 9e+01)) false true))

(fn ConstructionScript)